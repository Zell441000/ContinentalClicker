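; BP_MapLogic_Rail is a map-logic rail that links two slots and carries an adjustable level, shown on a text render.
; On BeginPlay it registers itself with each valid slot along with that end's priority.
; The construction script colors each rail half with a close, normal or far material chosen by priority, previewing it in the editor.
; It exposes its connected slots, level and LevelScene transform, and changes its level through a modify event.
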(event `self.ReceiveBeginPlay`
  (`|ExecutionSequence`
    (:`then_0`
      (`/Engine/EditorBlueprintResources/StandardMacros.IsValid` (`self.Slot_01`)
        (:`Is Valid`
          (message `/Game/GameLogis/MapLogic/Slot/BPI_Slot.Slot_AssignRail` (`self.Slot_01`) (`self.Priority_01`) self))))
    (:`then_1`
      (`/Engine/EditorBlueprintResources/StandardMacros.IsValid` (`self.Slot_02`)
        (:`Is Valid`
          (message `/Game/GameLogis/MapLogic/Slot/BPI_Slot.Slot_AssignRail` (`self.Slot_02`) (`self.Priority_02`) self))))))

(event `/Game/GameLogis/MapLogic/Rails/BPI_Rail.Rail_ModifyRailLevel`
  (params (AddLevel :type Boolean) (LevelQuantityToChange :type Integer))
  (set `self.Level` (+ (`self.Level`) (* LevelQuantityToChange (`KismetMathLibrary.SelectInt` 1 -1 AddLevel))))
  (`TextRenderComponent.K2_SetText` (`self.TextRender`) (`KismetTextLibrary.Conv_StringToText` (`KismetStringLibrary.Concat_StrStr` "lvl " (`KismetStringLibrary.Conv_IntToString` (`self.Level`))))))

(fn `Get_LevelSceneTransform`
  (returns (LvlScene :type "Transform Structure"))
  (return (`SceneComponent.K2_GetComponentToWorld` (`self.LevelScene`))))

(fn `Rail_GetConnectedSlots`
  (returns (Slots :type "Array of Actor Object Reference"))
  (return (`|MakeArray` (`self.Slot_01`) (`self.Slot_02`))))

(fn `Rail_GetRailLevel`
  (returns (Level :type Integer))
  (return (`self.Level`)))

(fn `UserConstructionScript`
  (`TextRenderComponent.K2_SetText` (`self.TextRender`) (`KismetTextLibrary.Conv_StringToText` (`KismetStringLibrary.Concat_StrStr` "lvl " (`KismetStringLibrary.Conv_IntToString` (`self.Level`)))))
  (`PrimitiveComponent.SetMaterial` (`self.Rail_01`) 0 (select `int` (`self.Priority_01`) :`0` "/Game/Materials/Test/MI_Rail_Close.MI_Rail_Close" :`1` "/Game/Materials/Test/MI_Rail_Normal.MI_Rail_Normal" :`2` "/Game/Materials/Test/MI_Rail_Far.MI_Rail_Far" :!type "MaterialInterface Object Reference"))
  (`PrimitiveComponent.SetMaterial` (`self.Rail_02`) 0 (select `int` (`self.Priority_02`) :`0` "/Game/Materials/Test/MI_Rail_Close.MI_Rail_Close" :`1` "/Game/Materials/Test/MI_Rail_Normal.MI_Rail_Normal" :`2` "/Game/Materials/Test/MI_Rail_Far.MI_Rail_Far" :!type "MaterialInterface Object Reference")))