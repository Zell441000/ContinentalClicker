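; Turn manager that cycles the game through Give Energy, Create, Dispatch and Consume resource phases via gameplay tags on the GameState's ability system.
; Each phase tag's removal starts the next; an external Chaos tag holds off Create until it clears.
; Resource phases process DT_Nations rows sequentially, sending a gameplay event per nation and awaiting its finish event before advancing.
; Startup retries each tick until the GameState and its ability system exist.
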(event `self.ReceiveBeginPlay`
  (`self.InitGameState`))

(event `InitGameState`
  (`/Engine/EditorBlueprintResources/StandardMacros.IsValid` (`GameplayStatics.GetGameState`)
    (:`Is Valid`
      (`/Engine/EditorBlueprintResources/StandardMacros.IsValid` (`AbilitySystemComponentBase.GetAbilitySystemComp` (`GameplayStatics.GetGameState`))
        (:`Is Valid`
          (`self.BindGameplayEvent`)
          (`self.BindStateTagManagement`)
          (`AbilitySystemComponentBase.SetGameplayTagCount` (`AbilitySystemComponentBase.GetAbilitySystemComp` (`GameplayStatics.GetGameState`)) (struct :`TagName` "Game.TurnState.GiveEnergy.IsCurrentState") 1))
        (:`Is Not Valid`
          (`KismetSystemLibrary.DelayUntilNextTick`)
          (`self.InitGameState`))))
    (:`Is Not Valid`
      (`KismetSystemLibrary.DelayUntilNextTick`)
      (`self.InitGameState`))))

(event `BindEventsForCreateRessources`
  (bind _currentnationrowindex (`self.CurrentNationRowIndex`))
  (`|ExecutionSequence`
    (:`then_0`
      (bind (_asynctaskproxy _tag _newcount) (`AbilityAsync_WaitGameplayTags.WaitGameplayTagsChangeOnActor` (`GameplayStatics.GetGameState`) (struct :`GameplayTags` (struct :`(TagName` "Game.TurnState.CreateRessources.IsCurrentState"))))
        (:`ChangeEvent`
          (if (`KismetMathLibrary.Conv_IntToBool` _newcount)
            (set `self.CurrentNationRowIndex` 0)
            (bind _outrownames (`DataTableFunctionLibrary.GetDataTableRowNames` "/Game/GameLogis/MainClasses/DataTable/Continent/DT_Nations.DT_Nations"))
            (`AbilitySystemBlueprintLibrary.SendGameplayEventToActor` (`GameplayStatics.GetGameState`) (struct :`TagName` "Game.TurnState.CreateRessources.CreateByNation_Event") (make `GameplayEventData` :`OptionalObject` (`|Utility_MakeVariableContainerNode` (`KismetStringLibrary.Conv_NameToString` (`|GetArrayItem` _outrownames (`self.CurrentNationRowIndex`))))))))))
    (:`then_1`
      (`AbilityAsync_WaitGameplayEvent.WaitGameplayEventToActor` (`GameplayStatics.GetGameState`) (struct :`TagName` "Game.TurnState.CreateRessources.FinishCreateByNation_Event")
        (:`EventReceived`
          (`/Engine/EditorBlueprintResources/StandardMacros.IncrementInt` (`self.CurrentNationRowIndex`)
            (:`  `
              (bind _outrownames_2 (`DataTableFunctionLibrary.GetDataTableRowNames` "/Game/GameLogis/MainClasses/DataTable/Continent/DT_Nations.DT_Nations"))
              (if (`KismetArrayLibrary.Array_IsValidIndex` _outrownames_2 _currentnationrowindex)
                (`AbilitySystemBlueprintLibrary.SendGameplayEventToActor` (`GameplayStatics.GetGameState`) (struct :`TagName` "Game.TurnState.CreateRessources.CreateByNation_Event") (make `GameplayEventData` :`OptionalObject` (`|Utility_MakeVariableContainerNode` (`KismetStringLibrary.Conv_NameToString` (`|GetArrayItem` _outrownames_2 _currentnationrowindex)))))
                (else
                  (`KismetSystemLibrary.Delay` 0.2)
                  (`AbilitySystemComponentBase.SetGameplayTagCount` (`AbilitySystemComponentBase.GetAbilitySystemComp` (`GameplayStatics.GetGameState`)) (struct :`TagName` "Game.TurnState.CreateRessources.IsCurrentState") 0))))))))))

(event `BindGameplayEvent`
  (`|ExecutionSequence`
    (:`then_0`
      (`self.BIndEventsForDispachRessources`))
    (:`then_1`
      (`self.BIndEventsForConsumeRessources`))
    (:`then_2`
      (`self.BindEventsForCreateRessources`))))

(event `BIndEventsForDispachRessources`
  (bind _currentnationrowindex (`self.CurrentNationRowIndex`))
  (`|ExecutionSequence`
    (:`then_0`
      (bind (_asynctaskproxy _tag _newcount) (`AbilityAsync_WaitGameplayTags.WaitGameplayTagsChangeOnActor` (`GameplayStatics.GetGameState`) (struct :`GameplayTags` (struct :`(TagName` "Game.TurnState.DispachRessources.IsCurrentState"))))
        (:`ChangeEvent`
          (if (`KismetMathLibrary.Conv_IntToBool` _newcount)
            (set `self.CurrentNationRowIndex` 0)
            (bind _outrownames (`DataTableFunctionLibrary.GetDataTableRowNames` "/Game/GameLogis/MainClasses/DataTable/Continent/DT_Nations.DT_Nations"))
            (`AbilitySystemBlueprintLibrary.SendGameplayEventToActor` (`GameplayStatics.GetGameState`) (struct :`TagName` "Game.TurnState.DispachRessources.DispatchBySlot_Event") (make `GameplayEventData` :`OptionalObject` (`|Utility_MakeVariableContainerNode` (`KismetStringLibrary.Conv_NameToString` (`|GetArrayItem` _outrownames (`self.CurrentNationRowIndex`))))))))))
    (:`then_1`
      (`AbilityAsync_WaitGameplayEvent.WaitGameplayEventToActor` (`GameplayStatics.GetGameState`) (struct :`TagName` "Game.TurnState.DispachRessources.FinishDispatchementByNation_Event")
        (:`EventReceived`
          (`/Engine/EditorBlueprintResources/StandardMacros.IncrementInt` (`self.CurrentNationRowIndex`)
            (:`  `
              (bind _outrownames_2 (`DataTableFunctionLibrary.GetDataTableRowNames` "/Game/GameLogis/MainClasses/DataTable/Continent/DT_Nations.DT_Nations"))
              (if (`KismetArrayLibrary.Array_IsValidIndex` _outrownames_2 _currentnationrowindex)
                (`AbilitySystemBlueprintLibrary.SendGameplayEventToActor` (`GameplayStatics.GetGameState`) (struct :`TagName` "Game.TurnState.DispachRessources.DispatchBySlot_Event") (make `GameplayEventData` :`OptionalObject` (`|Utility_MakeVariableContainerNode` (`KismetStringLibrary.Conv_NameToString` (`|GetArrayItem` _outrownames_2 _currentnationrowindex)))))
                (else
                  (`AbilitySystemBlueprintLibrary.SendGameplayEventToActor` (`GameplayStatics.GetGameState`) (struct :`TagName` "Game.TurnState.DispachRessources.FinishDispatchement_Event"))
                  (`KismetSystemLibrary.Delay` 0.2)
                  (`AbilitySystemComponentBase.SetGameplayTagCount` (`AbilitySystemComponentBase.GetAbilitySystemComp` (`GameplayStatics.GetGameState`)) (struct :`TagName` "Game.TurnState.DispachRessources.IsCurrentState") 0))))))))))

(event `BIndEventsForConsumeRessources`
  (bind _currentnationrowindex (`self.CurrentNationRowIndex`))
  (`|ExecutionSequence`
    (:`then_0`
      (bind (_asynctaskproxy _tag _newcount) (`AbilityAsync_WaitGameplayTags.WaitGameplayTagsChangeOnActor` (`GameplayStatics.GetGameState`) (struct :`GameplayTags` (struct :`(TagName` "Game.TurnState.ConsumeRessources.IsCurrentState"))))
        (:`ChangeEvent`
          (if (`KismetMathLibrary.Conv_IntToBool` _newcount)
            (set `self.CurrentNationRowIndex` 0)
            (bind _outrownames (`DataTableFunctionLibrary.GetDataTableRowNames` "/Game/GameLogis/MainClasses/DataTable/Continent/DT_Nations.DT_Nations"))
            (`AbilitySystemBlueprintLibrary.SendGameplayEventToActor` (`GameplayStatics.GetGameState`) (struct :`TagName` "Game.TurnState.ConsumeRessources.ConsumeByNation_Event") (make `GameplayEventData` :`OptionalObject` (`|Utility_MakeVariableContainerNode` (`KismetStringLibrary.Conv_NameToString` (`|GetArrayItem` _outrownames (`self.CurrentNationRowIndex`))))))))))
    (:`then_1`
      (`AbilityAsync_WaitGameplayEvent.WaitGameplayEventToActor` (`GameplayStatics.GetGameState`) (struct :`TagName` "Game.TurnState.ConsumeRessources.FinishConsumeByNation_Event")
        (:`EventReceived`
          (`/Engine/EditorBlueprintResources/StandardMacros.IncrementInt` (`self.CurrentNationRowIndex`)
            (:`  `
              (bind _outrownames_2 (`DataTableFunctionLibrary.GetDataTableRowNames` "/Game/GameLogis/MainClasses/DataTable/Continent/DT_Nations.DT_Nations"))
              (if (`KismetArrayLibrary.Array_IsValidIndex` _outrownames_2 _currentnationrowindex)
                (`AbilitySystemBlueprintLibrary.SendGameplayEventToActor` (`GameplayStatics.GetGameState`) (struct :`TagName` "Game.TurnState.ConsumeRessources.ConsumeByNation_Event") (make `GameplayEventData` :`OptionalObject` (`|Utility_MakeVariableContainerNode` (`KismetStringLibrary.Conv_NameToString` (`|GetArrayItem` _outrownames_2 _currentnationrowindex)))))
                (else
                  (`KismetSystemLibrary.Delay` 0.2)
                  (`AbilitySystemComponentBase.SetGameplayTagCount` (`AbilitySystemComponentBase.GetAbilitySystemComp` (`GameplayStatics.GetGameState`)) (struct :`TagName` "Game.TurnState.ConsumeRessources.IsCurrentState") 0))))))))))

(event `BindStateTagManagement`
  (`|ExecutionSequence`
    (:`then_0`
      (bind (_asynctaskproxy _tag _newcount) (`AbilityAsync_WaitGameplayTags.WaitGameplayTagsChangeOnActor` (`GameplayStatics.GetGameState`) (struct :`GameplayTags` (struct :`(TagName` "Game.TurnState.GiveEnergy.IsCurrentState"))))
        (:`ChangeEvent`
          (if (`KismetMathLibrary.Conv_IntToBool` _newcount)
            (`KismetSystemLibrary.PrintString` "Turn state : Give energy")
            (elif (not (`AbilitySystemComponentBase.HasGameplayTag` (`AbilitySystemComponentBase.GetAbilitySystemComp` (`GameplayStatics.GetGameState`)) (struct :`TagName` "Game.TurnState.ChaosState.IsINChaosState")))
              (`AbilitySystemComponentBase.SetGameplayTagCount` (`AbilitySystemComponentBase.GetAbilitySystemComp` (`GameplayStatics.GetGameState`)) (struct :`TagName` "Game.TurnState.CreateRessources.IsCurrentState") 1))))))
    (:`then_1`
      (bind (_asynctaskproxy_2 _tag_2 _newcount_2) (`AbilityAsync_WaitGameplayTags.WaitGameplayTagsChangeOnActor` (`GameplayStatics.GetGameState`) (struct :`GameplayTags` (struct :`(TagName` "Game.TurnState.CreateRessources.IsCurrentState"))))
        (:`ChangeEvent`
          (if (`KismetMathLibrary.Conv_IntToBool` _newcount_2)
            (`KismetSystemLibrary.PrintString` "Turn state : Create Ressources")
            (else
              (`AbilitySystemComponentBase.SetGameplayTagCount` (`AbilitySystemComponentBase.GetAbilitySystemComp` (`GameplayStatics.GetGameState`)) (struct :`TagName` "Game.TurnState.DispachRessources.IsCurrentState") 1))))))
    (:`then_2`
      (bind (_asynctaskproxy_3 _tag_3 _newcount_3) (`AbilityAsync_WaitGameplayTags.WaitGameplayTagsChangeOnActor` (`GameplayStatics.GetGameState`) (struct :`GameplayTags` (struct :`(TagName` "Game.TurnState.DispachRessources.IsCurrentState"))))
        (:`ChangeEvent`
          (if (`KismetMathLibrary.Conv_IntToBool` _newcount_3)
            (`KismetSystemLibrary.PrintString` "Turn state : Dispatch Ressources")
            (else
              (`AbilitySystemComponentBase.SetGameplayTagCount` (`AbilitySystemComponentBase.GetAbilitySystemComp` (`GameplayStatics.GetGameState`)) (struct :`TagName` "Game.TurnState.ConsumeRessources.IsCurrentState") 1))))))
    (:`then_3`
      (bind (_asynctaskproxy_4 _tag_4 _newcount_4) (`AbilityAsync_WaitGameplayTags.WaitGameplayTagsChangeOnActor` (`GameplayStatics.GetGameState`) (struct :`GameplayTags` (struct :`(TagName` "Game.TurnState.ConsumeRessources.IsCurrentState"))))
        (:`ChangeEvent`
          (if (`KismetMathLibrary.Conv_IntToBool` _newcount_4)
            (`KismetSystemLibrary.PrintString` "Turn state : Consume Ressources")
            (else
              (`AbilitySystemComponentBase.SetGameplayTagCount` (`AbilitySystemComponentBase.GetAbilitySystemComp` (`GameplayStatics.GetGameState`)) (struct :`TagName` "Game.TurnState.GiveEnergy.IsCurrentState") 1))))))
    (:`then_4`
      (bind (_asynctaskproxy_5 _tag_5 _newcount_5) (`AbilityAsync_WaitGameplayTags.WaitGameplayTagsChangeOnActor` (`GameplayStatics.GetGameState`) (struct :`GameplayTags` (struct :`(TagName` "Game.TurnState.ChaosState.IsINChaosState"))))
        (:`ChangeEvent`
          (if (not (`KismetMathLibrary.Conv_IntToBool` _newcount_5))
            (`AbilitySystemComponentBase.SetGameplayTagCount` (`AbilitySystemComponentBase.GetAbilitySystemComp` (`GameplayStatics.GetGameState`)) (struct :`TagName` "Game.TurnState.CreateRessources.IsCurrentState") 1)))))))

(fn `UserConstructionScript`)