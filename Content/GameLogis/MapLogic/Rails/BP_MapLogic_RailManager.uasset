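; BP_MapLogic_RailManager sequences the turn's resource dispatch phase, handling one nation at a time.
; On the GameState's start-dispatch event it resets the nation index and sends a dispatch-by-slot event carrying the first DT_Nations row name.
; Each finish-by-nation event advances the index and dispatches the next row, or sends the finish-dispatch event when none remain.
; All communication runs through tagged gameplay events on the GameState.
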(event `self.ReceiveBeginPlay`
  (bind _currentnationrowindex (`self.CurrentNationRowIndex`))
  (`|ExecutionSequence`
    (:`then_0`
      (`AbilityAsync_WaitGameplayEvent.WaitGameplayEventToActor` (`GameplayStatics.GetGameState`) (struct :`TagName` "Game.TurnState.DispachRessources.StartDispatchement_Event")
        (:`EventReceived`
          (set `self.CurrentNationRowIndex` 0)
          (bind _outrownames (`DataTableFunctionLibrary.GetDataTableRowNames` "/Game/GameLogis/MainClasses/DataTable/Continent/DT_Nations.DT_Nations"))
          (`AbilitySystemBlueprintLibrary.SendGameplayEventToActor` (`GameplayStatics.GetGameState`) (struct :`TagName` "Game.TurnState.DispachRessources.DispatchBySlot_Event") (make `GameplayEventData` :`OptionalObject` (`|Utility_MakeVariableContainerNode` (`KismetStringLibrary.Conv_NameToString` (`|GetArrayItem` _outrownames (`self.CurrentNationRowIndex`)))))))))
    (:`then_1`
      (`AbilityAsync_WaitGameplayEvent.WaitGameplayEventToActor` (`GameplayStatics.GetGameState`) (struct :`TagName` "Game.TurnState.DispachRessources.FinishDispatchementByNation_Event")
        (:`EventReceived`
          (`/Engine/EditorBlueprintResources/StandardMacros.IncrementInt` (`self.CurrentNationRowIndex`)
            (:`  `
              (bind _outrownames_2 (`DataTableFunctionLibrary.GetDataTableRowNames` "/Game/GameLogis/MainClasses/DataTable/Continent/DT_Nations.DT_Nations"))
              (if (`KismetArrayLibrary.Array_IsValidIndex` _outrownames_2 _currentnationrowindex)
                (`AbilitySystemBlueprintLibrary.SendGameplayEventToActor` (`GameplayStatics.GetGameState`) (struct :`TagName` "Game.TurnState.DispachRessources.DispatchBySlot_Event") (make `GameplayEventData` :`OptionalObject` (`|Utility_MakeVariableContainerNode` (`KismetStringLibrary.Conv_NameToString` (`|GetArrayItem` _outrownames_2 _currentnationrowindex)))))
                (else
                  (`AbilitySystemBlueprintLibrary.SendGameplayEventToActor` (`GameplayStatics.GetGameState`) (struct :`TagName` "Game.TurnState.DispachRessources.FinishDispatchement_Event")))))))))))

(fn `UserConstructionScript`)