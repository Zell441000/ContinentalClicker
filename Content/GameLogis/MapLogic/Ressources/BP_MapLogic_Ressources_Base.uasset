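; BP_MapLogic_Ressources_Base is a base map resource actor that displays a typed resource and can be moved across the map.
; Its construction script looks up its row in DT_Nations and applies that row's Color material to the cube, while RessourceGetType returns the row name.
; RessourceSetDeplacement starts a timed move, which Tick runs by lerping the actor transform to the target, optionally destroying the actor on arrival.
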(event `/Game/GameLogis/MapLogic/Ressources/BPI_Ressource.Ressource_SetDeplacement`
  (params (NewTransform :type "Transform Structure") (TimeToMove :type "Float (double-precision)") (DestroyOnFinish :type Boolean))
  (set `self.New Transform` NewTransform)
  (set `self.Time to Move` TimeToMove)
  (set `self.CurrentTimeDeplacement` 0.0)
  (set `self.OriginTransfrom` (`self.GetTransform`))
  (set `self.InDeplacement` true)
  (set `self.Destroy on Finish` DestroyOnFinish))

(event `self.ReceiveTick`
  (params (DeltaSeconds :type "Float (single-precision)"))
  (set `self.Delta Seconds` DeltaSeconds)
  (if (`self.InDeplacement`)
    (set `self.CurrentTimeDeplacement` (+ (`self.CurrentTimeDeplacement`) (`self.Delta Seconds`)))
    (`self.K2_SetActorTransform` (`KismetMathLibrary.TLerp` (`self.OriginTransfrom`) (`self.New Transform`) (`KismetMathLibrary.FClamp` (/ (`self.CurrentTimeDeplacement`) (`self.Time to Move`)))))
    (if (>= (/ (`self.CurrentTimeDeplacement`) (`self.Time to Move`)) 1.0)
      (set `self.InDeplacement` false)
      (if (`self.Destroy on Finish`)
        (`self.K2_DestroyActor`)))))

(fn `Ressource_GetType`
  (returns (Row :type Name))
  (return (`.RowName` (break `DataTableRowHandle` (`self.Row`)))))

(fn `UserConstructionScript`
  (bind _returnvalue (`|GetDataTableRow` "/Game/GameLogis/MainClasses/DataTable/Continent/DT_Nations.DT_Nations" (`.RowName` (break `DataTableRowHandle` (`self.Row`))))
    (:`then`
      (bind _returnvalue_2 (`KismetSystemLibrary.LoadAsset_Blocking` (`.Color_18_BD8431EC40A0E472A72F8EA304C11A98` (break `/Game/GameLogis/MainClasses/DataTable/Continent/Struct_Nations` _returnvalue))))
      (bind _asmaterial_instance (cast `MaterialInstance` _returnvalue_2))
      (`PrimitiveComponent.SetMaterial` (`self.Cube`) 0 _asmaterial_instance))))