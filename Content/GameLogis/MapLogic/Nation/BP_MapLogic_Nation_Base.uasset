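; Base map actor for a nation that sits on an assigned slot and produces its resource there, with its material taken from DT_Nations.
; Interacting recharges its energy component, marks it selected and grants one resource unless it is already the powered nation.
; Production drains energy unless selected, then requires remaining energy and, on corrupt slots, Thunas as cost except for row 0.
; A GameState gameplay tag listener clears selection at the GiveEnergy turn state.
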(event `self.ReceiveBeginPlay`
  (`self.InitGameState`)
  (`/Game/GameLogis/MapLogic/Nation/BP_Nation_Energy_Comp.InitWidget` (`self.BP_Nation_Energy_Comp`) (`WidgetComponent.GetWidget` (`self.Widget`))))

(event `InitGameState`
  (bind _returnvalue (`GameplayStatics.GetGameState`))
  (`/Engine/EditorBlueprintResources/StandardMacros.IsValid` _returnvalue
    (:`Is Valid`
      (`/Engine/EditorBlueprintResources/StandardMacros.IsValid` (`AbilitySystemComponentBase.GetAbilitySystemComp` _returnvalue)
        (:`Is Valid`
          (`self.BindGameplayEvents`))
        (:`Is Not Valid`
          (`KismetSystemLibrary.DelayUntilNextTick`)
          (`self.InitGameState`))))
    (:`Is Not Valid`
      (`KismetSystemLibrary.DelayUntilNextTick`)
      (`self.InitGameState`))))

(event `BindGameplayEvents`
  (`|ExecutionSequence`
    (:`then_1`
      (bind (_asynctaskproxy _tag _newcount) (`AbilityAsync_WaitGameplayTags.WaitGameplayTagsChangeOnActor` (`GameplayStatics.GetGameState`) (struct :`GameplayTags` (struct :`(TagName` "Game.TurnState.GiveEnergy.IsCurrentState"))))
        (:`ChangeEvent`
          (if (`KismetMathLibrary.Conv_IntToBool` _newcount)
            (set `self.IsSelected` false)))))))

(event `/Game/GameLogis/MapLogic/Nation/BPI_Nation.Nation_AssignSlot`
  (params (Slot :type "Actor Object Reference"))
  (bind _output_get (set `self.AssignedSlot` Slot))
  (`self.K2_SetActorLocation` (+ (`self.K2_GetActorLocation` _output_get) (0.0 0.0 50.0))))

(event `/Game/GameLogis/MapLogic/Nation/BPI_Nation.Nation_Interact`
  (`/Game/GameLogis/MapLogic/Nation/BP_Nation_Energy_Comp.RechargeEnergy` (`self.BP_Nation_Energy_Comp`))
  (set `self.IsSelected` true)
  (`AbilitySystemBlueprintLibrary.SendGameplayEventToActor` self (struct :`TagName` "Nation.State.Interact.Interact_Event"))
  (if (not (== (`AbilitySystemComponentBase.GetFirstObjectStoredWithGameplayTag` (`AbilitySystemComponentBase.GetAbilitySystemComp` (`GameplayStatics.GetGameState`)) (struct :`TagName` "Player.State.Interact.CurrentNationPowered_Object")) self))
    (message `/Game/GameLogis/MapLogic/Slot/BPI_Slot.Slot_ModifyRessourceQuantity` (`self.AssignedSlot`) (`.RowName` (break `DataTableRowHandle` (`self.DT_Row`))) true 1 false)))

(event `/Game/GameLogis/MapLogic/Nation/BPI_Nation.Nation_RechargeEnergy`
  (`/Game/GameLogis/MapLogic/Nation/BP_Nation_Energy_Comp.RechargeEnergy` (`self.BP_Nation_Energy_Comp`)))

(event `/Game/GameLogis/MapLogic/Nation/BPI_Nation.Nation_LaunchProduction`
  (`|ExecutionSequence`
    (:`then_0`
      (if (not (`self.IsSelected`))
        (`/Game/GameLogis/MapLogic/Nation/BP_Nation_Energy_Comp.RemoveOneEnergy` (`self.BP_Nation_Energy_Comp`))))
    (:`then_1`
      (if (`self.ProductionCondition`)
        (`|ExecutionSequence`
          (:`then_0`
            (`self.ProductionCostManager`))
          (:`then_1`
            (message `/Game/GameLogis/MapLogic/Slot/BPI_Slot.Slot_ModifyRessourceQuantity` (`self.AssignedSlot`) (`.RowName` (break `DataTableRowHandle` (`self.DT_Row`))) true (`self.ProductionLevel`) false)))))))

(fn `Nation_GetEnergyValue`
  (returns (Value :type Integer))
  (return (`/Game/GameLogis/MapLogic/Nation/BP_Nation_Energy_Comp.CurrentEnergyValue` (`self.BP_Nation_Energy_Comp`))))

(fn `Nation_GetRowName`
  (returns (Name :type Name))
  (return (`.RowName` (break `DataTableRowHandle` (`self.DT_Row`)))))

(fn `ProductionCondition`
  (returns (ReturnValue :type Boolean))
  (`|ExecutionSequence`
    (:`then_0`
      (if (not (> (`/Game/GameLogis/MapLogic/Nation/BP_Nation_Energy_Comp.CurrentEnergyValue` (`self.BP_Nation_Energy_Comp`)) 0))
        (return false)))
    (:`then_1`
      (bind _iscorrupt (message `/Game/GameLogis/MapLogic/Slot/BPI_Slot.Slot_GetIsCorrupt?` (`self.AssignedSlot`)))
      (if _iscorrupt
        (bind _ressources (message `/Game/GameLogis/MapLogic/Slot/BPI_Slot.Slot_GetRessources` (`self.AssignedSlot`)))
        (if (and (not (> (`BlueprintMapLibrary.Map_Find` _ressources "Thunas") 0)) (!= (`/Game/GameLogis/MainClasses/BPFL_ContinentalClicker.ConvertNameToInt` (`.RowName` (break `DataTableRowHandle` (`self.DT_Row`)))) 0))
          (return false))))
    (:`then_2`
      (return true))))

(fn `ProductionCostManager`
  (bind _iscorrupt (message `/Game/GameLogis/MapLogic/Slot/BPI_Slot.Slot_GetIsCorrupt?` (`self.AssignedSlot`)))
  (if _iscorrupt
    (if (!= (`/Game/GameLogis/MainClasses/BPFL_ContinentalClicker.ConvertNameToInt` (`.RowName` (break `DataTableRowHandle` (`self.DT_Row`)))) 0)
      (message `/Game/GameLogis/MapLogic/Slot/BPI_Slot.Slot_ModifyRessourceQuantity` (`self.AssignedSlot`) "Thunas" false 1 false))))

(fn `UserConstructionScript`
  (bind _returnvalue (`|GetDataTableRow` "/Game/GameLogis/MainClasses/DataTable/Continent/DT_Nations.DT_Nations" (`.RowName` (break `DataTableRowHandle` (`self.DT_Row`))))
    (:`then`
      (bind _returnvalue_2 (`KismetSystemLibrary.LoadAsset_Blocking` (`.Color_18_BD8431EC40A0E472A72F8EA304C11A98` (break `/Game/GameLogis/MainClasses/DataTable/Continent/Struct_Nations` _returnvalue))))
      (bind _asmaterial_instance (cast `MaterialInstance` _returnvalue_2))
      (`PrimitiveComponent.SetMaterial` (`self.Cube`) 0 _asmaterial_instance))))