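; Nation energy component that tracks a current energy value against a maximum, with events to refill it fully or spend one point while any remains.
; Each change sends an energy update gameplay event to the owner with old and new values in a variable container payload.
; It also pushes the current-to-max ratio to a widget through an update message; InitWidget stores that widget and starts it at zero.
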(event `RechargeEnergy`
  (set `self.LastValue` (`self.CurrentEnergyValue`))
  (set `self.CurrentEnergyValue` (`self.MaxEnergyValue`))
  (set `self.Variable CantainerForWidget` (`|Utility_MakeVariableContainerNode` (/ (`self.CurrentEnergyValue`) (`self.MaxEnergyValue`))))
  (`AbilitySystemBlueprintLibrary.SendGameplayEventToActor` (`self.GetOwner`) (struct :`TagName` "Nation.State.Energy.UpdateValue_Event") (make `GameplayEventData` :`OptionalObject` (`|Utility_MakeVariableContainerNode` (`KismetMathLibrary.Conv_IntToDouble` (`self.LastValue`)) (`KismetMathLibrary.Conv_IntToDouble` (`self.CurrentEnergyValue`)))))
  (message `/Game/GameLogis/MainClasses/Interface/BPI_Widget.WIdget_Update` (`self.WidgetRef`) (`self.Variable CantainerForWidget`)))

(event `InitWidget`
  (params (WidgetRef :type "Widget Object Reference"))
  (set `self.WidgetRef` WidgetRef)
  (set `self.Variable CantainerForWidget` (`|Utility_MakeVariableContainerNode` 0.0))
  (message `/Game/GameLogis/MainClasses/Interface/BPI_Widget.WIdget_Update` (`self.WidgetRef`) (`self.Variable CantainerForWidget`)))

(event `RemoveOneEnergy`
  (if (> (`self.CurrentEnergyValue`) 0)
    (set `self.LastValue` (`self.CurrentEnergyValue`))
    (`/Engine/EditorBlueprintResources/StandardMacros.DecrementInt` (`self.CurrentEnergyValue`)
      (:`  `
        (set `self.Variable CantainerForWidget` (`|Utility_MakeVariableContainerNode` (/ (`self.CurrentEnergyValue`) (`self.MaxEnergyValue`))))
        (`AbilitySystemBlueprintLibrary.SendGameplayEventToActor` (`self.GetOwner`) (struct :`TagName` "Nation.State.Energy.UpdateValue_Event") (make `GameplayEventData` :`OptionalObject` (`|Utility_MakeVariableContainerNode` (`KismetMathLibrary.Conv_IntToDouble` (`self.LastValue`)) (`KismetMathLibrary.Conv_IntToDouble` (`self.CurrentEnergyValue`)))))
        (message `/Game/GameLogis/MainClasses/Interface/BPI_Widget.WIdget_Update` (`self.WidgetRef`) (`self.Variable CantainerForWidget`))))))