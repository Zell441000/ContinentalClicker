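; Continental map slot that stores its assigned continent, resource quantities and prioritized rail connections.
; Quantity changes respawn or destroy per-type resource actors to match counts, spawning classes from DT_Continent at random offsets around the slot.
; It retries each tick until the GameState's ability system exists, then listens for the dispatch gameplay event.
; Dispatch is unfinished: it computes rail-level-capped amounts per resource but moves nothing.
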(event `self.ReceiveBeginPlay`
  (`self.BindGameplayEvent`))

(event `BindGameplayEvent`
  (`/Engine/EditorBlueprintResources/StandardMacros.IsValid` (`GameplayStatics.GetGameState`)
    (:`Is Valid`
      (`/Engine/EditorBlueprintResources/StandardMacros.IsValid` (`AbilitySystemComponentBase.GetAbilitySystemComp` (`GameplayStatics.GetGameState`))
        (:`Is Valid`
          (`AbilityAsync_WaitGameplayEvent.WaitGameplayEventToActor` (`GameplayStatics.GetGameState`) (struct :`TagName` "Game.TurnState.DispachRessources.Dispatch_Event")
            (:`EventReceived`
              (`self.DIspatchEvent`))))
        (:`Is Not Valid`
          (`KismetSystemLibrary.DelayUntilNextTick`)
          (`self.BindGameplayEvent`))))
    (:`Is Not Valid`
      (`KismetSystemLibrary.DelayUntilNextTick`)
      (`self.BindGameplayEvent`))))

(event `/Game/GameLogis/MapLogic/Slot/BPI_ContinentalSlot.Slot_AssignContinent`
  (params (Continent :type "Actor Object Reference"))
  (set `self.AssignedContinent` Continent))

(event `/Game/GameLogis/MapLogic/Slot/BPI_ContinentalSlot.Slot_ModifyRessourceQuantity`
  (params (RessourceName :type Name) (Add :type Boolean) (Quantity :type Integer))
  (`BlueprintMapLibrary.Map_Add` (`self.RessourcesOnSlot`) RessourceName (+ (`BlueprintMapLibrary.Map_Find` (`self.RessourcesOnSlot`) RessourceName) (* Quantity (`KismetMathLibrary.SelectInt` 1 -1 Add))))
  (`self.UpdateRessourceActors`))

(event `UpdateRessourceActors`
  (`self.ManageRessourceActorSpawn`))

(event `/Game/GameLogis/MapLogic/Slot/BPI_ContinentalSlot.Slot_AssignRail`
  (params (Prio :type Integer) (Rail :type "Actor Object Reference"))
  (`BlueprintMapLibrary.Map_Add` (`self.RailsConnected`) Prio Rail))

(event `DispatchEvent`
  (bind _keys (`BlueprintMapLibrary.Map_Keys` (`self.RessourcesOnSlot`)))
  (for _array_element _keys
    (`self.DispatchRessourceByType` _array_element)))

(fn `ConvertNameToInt`
  (params (Name :type Name))
  (returns (num :type Integer))
  (switch `name` Name
    (:`Thunas`
      (return 0))
    (:`Transport`
      (return 1))
    (:`Sciences`
      (return 2))
    (:`Social`
      (return 3))
    (:`Construction`
      (return 4))))

(fn `DispatchRessourceByType`
  (params (Type :type "Name (by ref)"))
  (locals (CurrentRail :type "Actor Object Reference") (RessourceToRemove :type Integer :default 0) (CurrentLevel :type Integer :default 0))
  (bind _keys (`BlueprintMapLibrary.Map_Keys` (`self.RailsConnected`)))
  (for _array_element _keys
    (`|ExecutionSequence`
      (:`then_0`
        (bind _output_get (set `local.CurrentRail` (`BlueprintMapLibrary.Map_Find` (`self.RailsConnected`) _array_element)))
        (bind _level (message `/Game/GameLogis/MapLogic/Rails/BPI_Rail.Rail_GetRailLevel` _output_get))
        (bind _output_get_2 (set `local.CurrentLevel` _level))
        (set `local.RessourceToRemove` (`KismetMathLibrary.Min` _output_get_2 (`BlueprintMapLibrary.Map_Find` (`self.RessourcesOnSlot`) (`local.Type`))))))))

(fn `ManageRessourceActorSpawn`
  (locals (CurrentRow :type Name) (Diff :type Integer) (IndexToRemove :type Integer :default 0))
  (bind _keys (`BlueprintMapLibrary.Map_Keys` (`self.RessourcesOnSlot`)))
  (for _array_element _keys
    (set `local.CurrentRow` _array_element)
    (bind _thunasactors (`self.GetActorArrayWithType` (`local.CurrentRow`))
      (:`OutputPin`
        (bind _output_get (set `local.Diff` (- (`BlueprintMapLibrary.Map_Find` (`self.RessourcesOnSlot`) (`local.CurrentRow`)) (`KismetArrayLibrary.Array_Length` _thunasactors))))
        (`/Engine/EditorBlueprintResources/StandardMacros.CompareInt` _output_get
          (:`>`
            (for _ (range (`local.Diff`))
              (bind _returnvalue (`|GetDataTableRow` "/Game/GameLogis/MainClasses/DataTable/Continent/DT_Continent.DT_Continent" (`local.CurrentRow`))
                (:`then`
                  (bind _returnvalue_2 (`KismetSystemLibrary.LoadClassAsset_Blocking` (`.RessourceClass_21_46A2A14040202B16103EA18C83CEABFE` (break `/Game/GameLogis/MainClasses/DataTable/Continent/Struct_Continent` _returnvalue))))
                  (bind _asactor (castclass `Actor` _returnvalue_2))
                  (bind _returnvalue_3 (`|SpawnActorFromClass` _asactor (`KismetMathLibrary.MakeTransform` (+ (`self.K2_GetActorLocation`) (`KismetMathLibrary.MakeVector` (`KismetMathLibrary.RandomFloatInRange` -500.0 500.0) (`KismetMathLibrary.RandomFloatInRange` -200.0 200.0) 100.0)) (`KismetMathLibrary.MakeRotator` 0.0 0.0 (`KismetMathLibrary.RandomFloatInRange` 0.0 360.0))) "Undefined" "MultiplyWithRoot" null null))
                  (bind _thunasactors_2 (`self.GetActorArrayWithType` (`local.CurrentRow`))
                    (:`OutputPin`
                      (`KismetArrayLibrary.Array_Add` _thunasactors_2 _returnvalue_3)))))))
          (:`<`
            (for _ (range (`KismetMathLibrary.Abs_Int` (`local.Diff`)))
              (bind _thunasactors_3 (`self.GetActorArrayWithType` (`local.CurrentRow`))
                (:`OutputPin`
                  (set `local.IndexToRemove` (`KismetMathLibrary.RandomIntegerInRange` 0 (- (`KismetArrayLibrary.Array_Length` _thunasactors_3) 1)))
                  (bind _thunasactors_4 (`self.GetActorArrayWithType` (`local.CurrentRow`))
                    (:`OutputPin`
                      (`self.K2_DestroyActor` (`|GetArrayItem` _thunasactors_4))
                      (bind _thunasactors_5 (`self.GetActorArrayWithType` (`local.CurrentRow`))
                        (:`OutputPin`
                          (`KismetArrayLibrary.Array_Remove` _thunasactors_5 (`local.IndexToRemove`)))))))))))))))

(fn `Slot_GetAssignedContinent`
  (returns (Continent :type "Actor Object Reference"))
  (return (`self.AssignedContinent`)))

(fn `UserConstructionScript`)