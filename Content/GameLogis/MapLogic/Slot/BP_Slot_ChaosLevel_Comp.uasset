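; Slot component that tracks a chaos level and defines escalating penalties for the slot.
; It follows the assigned nation through gameplay events: interactions raise the level, and energy depletion calls ChaosEvent, which is an empty stub.
; The level sets layer tags through nested threshold checks that test the first threshold first.
; ChaosEventManager, uncalled here, maps those tags to destroying resources, downgrading rails or marking the slot unusable.
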(event `self.ReceiveBeginPlay`
  (`self.BindGameplayEvent`))

(event `BindGameplayEvent`
  (bind (_asynctaskproxy _payload) (`AbilityAsync_WaitGameplayEvent.WaitGameplayEventToActor` (`self.GetOwner`) (struct :`TagName` "Slot.State.AssignedNation.Change_Event"))
    (:`EventReceived`
      (bind _asactor (cast `Actor` (`.OptionalObject` (break `GameplayEventData` _payload))))
      (set `self.NationAssigned` _asactor)
      (`self.BindEventOnNation`))))

(event `BindEventOnNation`
  (bind _async_actionupdateenergy (`self.Async ActionUpdateEnergy`))
  (`|ExecutionSequence`
    (:`then_0`
      (`/Engine/EditorBlueprintResources/StandardMacros.IsValid` _async_actionupdateenergy
        (:`Is Valid`
          (`AbilityAsync.EndAction` _async_actionupdateenergy))))
    (:`then_1`
      (`/Engine/EditorBlueprintResources/StandardMacros.IsValid` (`self.NationAssigned`)
        (:`Is Valid`
          (`|ExecutionSequence`
            (:`then_0`
              (bind (_asynctaskproxy _payload) (`AbilityAsync_WaitGameplayEvent.WaitGameplayEventToActor` (`self.NationAssigned`) (struct :`TagName` "Nation.State.Energy.UpdateValue_Event"))
                (:`then`
                  (set `self.Async ActionUpdateEnergy` _asynctaskproxy))
                (:`EventReceived`
                  (bind _asvariable_container (cast `VariableContainer` (`.OptionalObject` (break `GameplayEventData` _payload))))
                  (bind (_oldvalue _newvalue) (`|Utility_BreakVariableContainerNode` _asvariable_container))
                  (if (and (> _oldvalue 0.0) (<= _newvalue 0.0))
                    (`self.ChaosEvent`)))))
            (:`then_1`
              (`AbilityAsync_WaitGameplayEvent.WaitGameplayEventToActor` (`self.NationAssigned`) (struct :`TagName` "Nation.State.Interact.Interact_Event")
                (:`EventReceived`
                  (`self.IncreaseChaosLevel`))))))))))

(event `ChaosEvent`)

(event `IncreaseChaosLevel`
  (`self.ChaosLevelIncreaseManager`))

(fn `ChaosEventManager`
  (if (`AbilitySystemComponentBase.HasGameplayTag` (`AbilitySystemComponentBase.GetAbilitySystemComp` (`self.GetOwner`)) (struct :`TagName` "Slot.State.ChaosLevel.IsInFirstLayer"))
    (`AbilitySystemBlueprintLibrary.SendGameplayEventToActor` (`self.GetOwner`) (struct :`TagName` "Slot.Action.ChaosAction.DestroyAllRessources_Event"))
    (elif (`AbilitySystemComponentBase.HasGameplayTag` (`AbilitySystemComponentBase.GetAbilitySystemComp` (`self.GetOwner`)) (struct :`TagName` "Slot.State.ChaosLevel.IsInSecondLayer"))
      (`AbilitySystemBlueprintLibrary.SendGameplayEventToActor` (`self.GetOwner`) (struct :`TagName` "Slot.Action.ChaosAction.RailsLevelDown_Event"))
      (elif (`AbilitySystemComponentBase.HasGameplayTag` (`AbilitySystemComponentBase.GetAbilitySystemComp` (`self.GetOwner`)) (struct :`TagName` "Slot.State.ChaosLevel.IsInThirdLayer"))
        (`AbilitySystemComponentBase.SetGameplayTagCount` (`AbilitySystemComponentBase.GetAbilitySystemComp` (`self.GetOwner`)) (struct :`TagName` "Slot.State.IsInusable") 1)))))

(fn `ChaosLevelIncreaseManager`
  (if (< (`self.CurrentChaosLevel`) (`self.ChaosThirdThreshold`))
    (`/Engine/EditorBlueprintResources/StandardMacros.IncrementInt` (`self.CurrentChaosLevel`)
      (:`  `
        (if (>= (`self.CurrentChaosLevel`) (`self.ChaosFirstThreshold`))
          (if (not (`AbilitySystemComponentBase.HasGameplayTag` (`AbilitySystemComponentBase.GetAbilitySystemComp` (`self.GetOwner`)) (struct :`TagName` "Slot.State.ChaosLevel.IsInFirstLayer")))
            (`AbilitySystemComponentBase.SetGameplayTagCount` (`AbilitySystemComponentBase.GetAbilitySystemComp` (`self.GetOwner`)) (struct :`TagName` "Slot.State.ChaosLevel.IsInFirstLayer") 1))
          (elif (>= (`self.CurrentChaosLevel`) (`self.ChaosSecondThreshold`))
            (if (not (`AbilitySystemComponentBase.HasGameplayTag` (`AbilitySystemComponentBase.GetAbilitySystemComp` (`self.GetOwner`)) (struct :`TagName` "Slot.State.ChaosLevel.IsInSecondLayer")))
              (`AbilitySystemComponentBase.SetGameplayTagCount` (`AbilitySystemComponentBase.GetAbilitySystemComp` (`self.GetOwner`)) (struct :`TagName` "Slot.State.ChaosLevel.IsInSecondLayer") 1))
            (elif (>= (`self.CurrentChaosLevel`) (`self.ChaosThirdThreshold`))
              (if (not (`AbilitySystemComponentBase.HasGameplayTag` (`AbilitySystemComponentBase.GetAbilitySystemComp` (`self.GetOwner`)) (struct :`TagName` "Slot.State.ChaosLevel.IsInThirdLayer")))
                (`AbilitySystemComponentBase.SetGameplayTagCount` (`AbilitySystemComponentBase.GetAbilitySystemComp` (`self.GetOwner`)) (struct :`TagName` "Slot.State.ChaosLevel.IsInThirdLayer") 1)))))))))