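; BP_MapLogic_Continent_Base is a base continent actor on the game map, configured by a row in DT_Continent.
; Its construction script loads that row's color material synchronously and applies it to the cube.
; Assigning a slot stores it and teleports the continent just above it.
; Interacting tells the assigned slot to add a fixed quantity of the resource named after the continent's row.
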(event `/Game/GameLogis/MapLogic/Continent/BPI_Continent.Continent_AssignSlot`
  (params (Slot :type "Actor Object Reference"))
  (bind _output_get (set `self.AssignedSlot` Slot))
  (`self.K2_SetActorLocation` (+ (`self.K2_GetActorLocation` _output_get) (0.0 0.0 50.0))))

(event `/Game/GameLogis/MapLogic/Continent/BPI_Continent.Continent_Interact`
  (message `/Game/GameLogis/MapLogic/ContinentalSlot/BPI_ContinentalSlot.ContinentSlot_ModifyRessourceQuantity` (`self.AssignedSlot`) (`.RowName` (break `DataTableRowHandle` (`self.DT_Row`))) true 2))

(fn `Continent_GetRowName`
  (returns (Name :type Name))
  (return (`.RowName` (break `DataTableRowHandle` (`self.DT_Row`)))))

(fn `UserConstructionScript`
  (bind _returnvalue (`|GetDataTableRow` "/Game/GameLogis/MainClasses/DataTable/Continent/DT_Continent.DT_Continent" (`.RowName` (break `DataTableRowHandle` (`self.DT_Row`))))
    (:`then`
      (bind _returnvalue_2 (`KismetSystemLibrary.LoadAsset_Blocking` (`.Color_18_BD8431EC40A0E472A72F8EA304C11A98` (break `/Game/GameLogis/MainClasses/DataTable/Continent/Struct_Continent` _returnvalue))))
      (bind _asmaterial_instance (cast `MaterialInstance` _returnvalue_2))
      (`PrimitiveComponent.SetMaterial` (`self.Cube`) 0 _asmaterial_instance))))