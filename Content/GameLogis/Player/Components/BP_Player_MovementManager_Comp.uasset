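; BP_Player_MovementManager_Comp is a player component that handles mouse-driven camera zoom and panning.
; Mouse wheel input accumulates into an inverted, sensitivity-scaled field of view, applied without clamping to the owner's first camera tagged "Camera".
; While the right mouse button is held, mouse movement offsets the owning actor in world XY, with X inverted, scaled by movement sensitivity and without sweep.
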(event `InputAxisKey|MouseWheelAxis`
  (params (AxisValue :type "Float (single-precision)"))
  (set `self.In Field Of View` (+ (`self.In Field Of View`) (* (* AxisValue -1.0) (`self.Sensibility`))))
  (`CameraComponent.SetFieldOfView` (`|GetArrayItem` (`Actor.GetComponentsByTag` (`self.GetOwner`) "/Script/Engine.CameraComponent" "Camera")) (`self.In Field Of View`)))

(event `InputVectorAxis|Mouse2D`
  (params (AxisValue :type "Vector Structure"))
  (if (`self.RightMouseInputPressed`)
    (`Actor.K2_SetActorLocation` (`self.GetOwner`) (+ (`Actor.K2_GetActorLocation` (`self.GetOwner`)) (* (`KismetMathLibrary.MakeVector` (* (.x AxisValue) -1.0) (.y AxisValue)) (`self.MovementSensibility`))) false false)))

(event `Key|RightMouseButton`
  (params (Key :type "Key Structure"))
  (:`Pressed`
    (set `self.RightMouseInputPressed` true))
  (:`Released`
    (set `self.RightMouseInputPressed` false)))