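; Player interaction component that handles clicks on continents and continental slots, assigning a selected continent to a free slot.
; A gameplay event on the GameState carries a row name, and the matching continent is stored as a tagged object in its ability system component.
; Click line traces route by interface: slots link with the stored continent, then clear it and send an update event, while continents receive an interact message.
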(event `self.ReceiveBeginPlay`
  (bind (_asynctaskproxy _payload) (`AbilityAsync_WaitGameplayEvent.WaitGameplayEventToActor` (`GameplayStatics.GetGameState`) (struct :`TagName` "Player.State.UI_Interaction.UpdateSelectedContinent_Event"))
    (:`EventReceived`
      (bind _asvariable_container (cast `VariableContainer` (`.OptionalObject` (break `GameplayEventData` _payload))))
      (`self.SetSelectedContinent` (`|Utility_BreakVariableContainerNode` _asvariable_container)))))

(event `EnhancedInput|/Game/GameLogis/Input/IA_Click`
  (params (ActionValue :type Boolean) (ElapsedSeconds :type "Float (double-precision)") (TriggeredSeconds :type "Float (double-precision)") (InputAction :type "InputAction Object Reference" :default "/Game/GameLogis/Input/IA_Click.IA_Click"))
  (bind (_worldlocation _worlddirection) (`PlayerController.DeprojectMousePositionToWorld` (`GameplayStatics.GetPlayerController` 0)))
  (:`Completed`
    (bind (_outhit _returnvalue) (`KismetSystemLibrary.LineTraceSingle` _worldlocation (+ _worldlocation (* _worlddirection 5000.0)) "TraceTypeQuery3" false (`|MakeArray` (`self.GetOwner`))))
    (if _returnvalue
      (set `self.CurrentActorClicked` (`.HitActor` (`GameplayStatics.BreakHitResult` _outhit)))
      (if (`KismetSystemLibrary.DoesImplementInterface` (`self.CurrentActorClicked`) "/Game/GameLogis/MapLogic/Slot/BPI_ContinentalSlot.BPI_ContinentalSlot_C")
        (`self.InteractWithSlot` (`self.CurrentActorClicked`))
        (elif (`KismetSystemLibrary.DoesImplementInterface` (`self.CurrentActorClicked`) "/Game/GameLogis/MapLogic/Nation/BPI_Continent.BPI_Continent_C")
          (`self.InteractWithContinent` (`self.CurrentActorClicked`)))))))

(event `InteractWithSlot`
  (params (SLot :type "Actor Object Reference"))
  (`self.SlotInteractionManager` SLot))

(event `InteractWithContinent`
  (params (Continent :type "Actor Object Reference"))
  (`self.ContinentInteractionManager` Continent)
  (`KismetSystemLibrary.PrintString` "Hello"))

(fn `CanAssignSlot?`
  (params (Slot :type "Actor Object Reference"))
  (returns (Yes :type Boolean))
  (bind _continent (message `/Game/GameLogis/MapLogic/Slot/BPI_ContinentalSlot.Slot_GetAssignedContinent` Slot))
  (`/Engine/EditorBlueprintResources/StandardMacros.IsValid` _continent
    (:`Is Valid`
      (return false))
    (:`Is Not Valid`
      (return true))))

(fn `ContinentInteractionManager`
  (params (Actor :type "Actor Object Reference"))
  (message `/Game/GameLogis/MapLogic/Nation/BPI_Continent.Continent_Interact` Actor))

(fn `SetSelectedContinent`
  (params (RowName :type String))
  (locals (CurrentContinent :type "Actor Object Reference"))
  (bind _outactors (`GameplayStatics.GetAllActorsWithInterface` "/Game/GameLogis/MapLogic/Nation/BPI_Continent.BPI_Continent_C"))
  (for _array_element _outactors
    (bind _output_get (set `local.CurrentContinent` _array_element))
    (bind _name (message `/Game/GameLogis/MapLogic/Nation/BPI_Continent.Continent_GetRowName` _output_get))
    (if (== _name (`KismetStringLibrary.Conv_StringToName` (`local.RowName`)))
      (`AbilitySystemComponentBase.SetObjectStoredWithGameplayTag` (`AbilitySystemComponentBase.GetAbilitySystemComp` (`GameplayStatics.GetGameState`)) (struct :`TagName` "Player.State.UI_Interaction.SelectedContinent_Object") (`local.CurrentContinent`))
      (return))))

(fn `SlotInteractionManager`
  (params (InteractedSlot :type "Actor Object Reference"))
  (locals (SelectedContinent :type "Object Object Reference"))
  (if (`self.CanAssignSlot?` InteractedSlot)
    (`|ExecutionSequence`
      (:`then_0`
        (set `local.SelectedContinent` (`AbilitySystemComponentBase.GetFirstObjectStoredWithGameplayTag` (`AbilitySystemComponentBase.GetAbilitySystemComp` (`GameplayStatics.GetGameState`)) (struct :`TagName` "Player.State.UI_Interaction.SelectedContinent_Object")))
        (`/Engine/EditorBlueprintResources/StandardMacros.IsValid` (`local.SelectedContinent`)
          (:`Is Valid`
            (if (not (`KismetSystemLibrary.DoesImplementInterface` (`local.SelectedContinent`) "/Game/GameLogis/MapLogic/Nation/BPI_Continent.BPI_Continent_C"))
              (return)))
          (:`Is Not Valid`
            (return))))
      (:`then_1`
        (message `/Game/GameLogis/MapLogic/Nation/BPI_Continent.Continent_AssignSlot` (`local.SelectedContinent`) (`local.InteractedSlot`))
        (message `/Game/GameLogis/MapLogic/Slot/BPI_ContinentalSlot.Slot_AssignContinent` (`local.InteractedSlot`) (cast `Actor` (`local.SelectedContinent`) :!pure true)))
      (:`then_2`
        (`AbilitySystemComponentBase.ClearObjectsStoredWithGameplayTag` (`AbilitySystemComponentBase.GetAbilitySystemComp` (`GameplayStatics.GetGameState`)) (struct :`TagName` "Player.State.UI_Interaction.SelectedContinent_Object"))
        (`AbilitySystemBlueprintLibrary.SendGameplayEventToActor` (`GameplayStatics.GetGameState`) (struct :`TagName` "Player.State.UI_Interaction.UpdateSelectedContinent_Event"))))))